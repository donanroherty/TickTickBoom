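; Player controller that owns a custom camera, opens the pause menu and gives access to the game board.
; On BeginPlay it spawns a BP_CameraActor as the view target and forwards focus target changes to it.
; The construction script also sets the camera reference from a child actor component, which BeginPlay then overwrites.
; Pause input calls BP_HUD, and GetGameBoard fetches the board from BP_GameMode.
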(event `self.ReceiveBeginPlay`
  (bind _returnvalue (`|SpawnActorFromClass` "/Game/Blueprint/BP_CameraActor.BP_CameraActor_C" (`KismetMathLibrary.MakeTransform` (0.0 0.0 0.0)) "AlwaysSpawn" "OverrideRootScale")) ; Spawn the custom camera actor...
  (bind _output_get (set `self.CameraActor` _returnvalue))
  (`self.SetViewTargetWithBlend` _output_get) ; And set it as the view target
)

(event `SetCameraFocusTarget`
  (params (NewFocusTarget :type "Actor Object Reference"))
  (`/Game/Blueprint/BP_CameraActor.SetFocusTarget` (`self.CameraActor`) NewFocusTarget))

(event `InputAction|PauseGame`
  (params (Key :type "Key Structure" :default "AnyKey"))
  (:`Pressed`
    (`/Game/Blueprint/BP_HUD.OpenPauseMenu` (cast `/Game/Blueprint/BP_HUD` (`self.GetHUD`) :!pure true))))

(fn `GetGameBoard`
  (returns (OutGB :type "/Game/Blueprint/BP_GameBoard Object Reference"))
  (return (`/Game/Blueprint/BP_GameMode.GetGameBoard` (cast `/Game/Blueprint/BP_GameMode` (`GameplayStatics.GetGameMode`) :!pure true))))

(fn `UserConstructionScript`
  (bind _returnvalue (`AddComponent|Child Actor Component_18803`))
  (set `self.CameraActor` (cast `/Game/Blueprint/BP_CameraActor` (`ChildActorComponent.ChildActor` _returnvalue) :!pure true)))