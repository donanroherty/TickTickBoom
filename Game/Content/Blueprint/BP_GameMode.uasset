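; Game mode that runs a stage-based button-press game, from tutorial through stage completion, death and game completion.
; At BeginPlay it spawns a board per data table row, spacing them along Y by actor bounds, and focuses the camera on the first.
; Each stage activates its board and starts a pre-cycle; success saves the high score and notifies the HUD, with dialog dismissal advancing stages.
; Short circuits are gated by remaining count and board state.
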(event `self.ReceiveBeginPlay`
  (`self.SpawnGameBoards`) ; Spawns all gameboards in a row from left to right
  (`TTBPlayerController.SetCameraFocusTarget` (cast `TTBPlayerController` (`GameplayStatics.GetPlayerController` 0) :!pure true) (`self.GetGameBoard`))
  (`KismetSystemLibrary.Delay` 3.0)
  (if (not (`/Game/Blueprint/BP_GameInstance.HideTutorial` (cast `/Game/Blueprint/BP_GameInstance` (`GameplayStatics.GetGameInstance`) :!pure true)))
    (`/Game/Blueprint/BP_HUD.ShowTutorial` (`self.GetHud`)))
  (`self.StartCurrentStage`))

(event `StartCurrentStage`
  ;[1 1 1] Manage stage switching
  (`TTBPlayerController.SetCameraFocusTarget` (cast `TTBPlayerController` (`GameplayStatics.GetPlayerController` 0) :!pure true) (`self.GetGameBoard`))
  (`/Game/Blueprint/BP_GameBoard.ActivateBoard` (`self.GetGameBoard`))
  (`KismetSystemLibrary.Delay` 2.0)
  (`/Game/Blueprint/BP_GameBoard.BeginPreCycle` (`self.GetGameBoard`)))

(event `IncrementStage`
  ;[1 1 1] Manage stage switching
  (`/Engine/EditorBlueprintResources/StandardMacros.IsValid` (`self.GetGameBoard`)
    (:`Is Valid`
      (`/Game/Blueprint/BP_GameBoard.DeactivateBoard` (`self.GetGameBoard`)) ; Deactivate previous board if it exists
    )
    (:`Is Not Valid`
      _))
  (`/Engine/EditorBlueprintResources/StandardMacros.IncrementInt` (`self.CurrentStage`)
    (:`  `
      (`self.StartCurrentStage`))))

(event `OnStageCompleteDialogDismissed`
  ;[1 1 1] Manage stage switching
  (`self.IncrementStage`))

(event `OnStageSucess`
  (bind _hud (`self.GetHud`))
  ;[1 1 1] manage stage success/failure
  (`KismetSystemLibrary.Delay` 1.0)
  (`/Game/Blueprint/BP_GameInstance.SetHighScore` (cast `/Game/Blueprint/BP_GameInstance` (`GameplayStatics.GetGameInstance`) :!pure true) (+ (`self.CurrentStage`) 1))
  (if (> (+ (`self.CurrentStage`) 1) (`self.MaxStageCount`))
    (`/Game/Blueprint/BP_HUD.OnGameComplete` _hud)
    (else
      (`/Game/Blueprint/BP_HUD.OnStageComplete` _hud))))

(event `OnStageFailed`
  ;[1 1 1] manage stage success/failure
  (`KismetSystemLibrary.Delay` 3.0)
  (`/Game/Blueprint/BP_HUD.OnDeath` (`self.GetHud`)))

(event `ShortCircuit`
  ;[1 1 1] Test short circuit viability
  (if (and (> (`self.AvailableShortCircuits`) 0) (`|EnumEquality` (`/Game/Blueprint/BP_GameBoard.BoardState` (`self.GetGameBoard`)) "NewEnumerator2"))
    (`self.OnShortCircuit`)))

(fn `GetGameBoard`
  (returns (OutGB :type "/Game/Blueprint/BP_GameBoard Object Reference"))
  (return (`|GetArrayItem` (`self.Gameboards`) (`self.CurrentStage`))))

(fn `GetHud`
  (returns (Hud :type "/Game/Blueprint/BP_HUD Object Reference"))
  (return (cast `/Game/Blueprint/BP_HUD` (`PlayerController.GetHUD` (`GameplayStatics.GetPlayerController` 0)) :!pure true)))

(fn `GetMaxStageCount`
  (returns (BoardCount :type Integer))
  (bind _outrownames (`DataTableFunctionLibrary.GetDataTableRowNames` "/Game/Blueprint/Data/GameBoard_DataTable.Gameboard_DataTable"))
  (return (`KismetArrayLibrary.Array_Length` _outrownames)))

(fn `SpawnGameBoards`
  (locals (SpawnLoc :type "Vector Structure"))
  (bind _gameboards (`self.Gameboards`))
  (bind _output (`|GetArrayItem` _gameboards (- (`KismetArrayLibrary.Array_LastIndex` _gameboards) 1)))
  (for _index (range (`self.GetMaxStageCount`))
    (bind _returnvalue (`|GetDataTableRow` "/Game/Blueprint/Data/GameBoard_DataTable.Gameboard_DataTable" (`KismetStringLibrary.Conv_StringToName` (`KismetStringLibrary.Conv_IntToString` _index)))
      (:`then`
        (bind _returnvalue_2 (`|SpawnActorFromClass` "/Game/Blueprint/BP_GameBoard.BP_GameBoard_C" (`KismetMathLibrary.MakeTransform` (0.0 0.0 0.0)) "AlwaysSpawn" "OverrideRootScale" null _returnvalue null)) ; Always spawn at 0.  Game boards are moved after when we know the bounds of this new gameboard
        (`KismetArrayLibrary.Array_Add` (`self.Gameboards`) _returnvalue_2)
        (if (> _index 0)
          (`self.K2_SetActorLocation` _returnvalue_2 (+ (`self.K2_GetActorLocation` _output) (`KismetMathLibrary.MakeVector` 0.0 (+ (.y (`.BoxExtent` (`self.GetActorBounds` _output false))) (.y (`.BoxExtent` (`self.GetActorBounds` _returnvalue_2 false))) (`self.BoardSpacing`)))) false false))))))

(fn `UserConstructionScript`)