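; BP_GameBoard runs a shell-game stage: track the safe button as the grid shuffles, then click it to avoid an explosion.
; The construction script builds the button grid, walls and gates from GameboardData.
; Timer-driven phases flash and pick the safe button, count down, then cycle random rows or columns, biased toward the safe one.
; Wrapping buttons teleport to the opposite side while spawned proxies exit, and results go to BP_GameMode.
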(event Custom|Cycle
  (bind _gameboarddata (Variables|Default|GetGameboardData))
  (bind _cyclecount (Utilities|Struct|BreakGameboardData _gameboarddata))
  ;[1 1 1] Manage button cycling
  (CallFunction|CycleButtons)
  (bind _counter (Utilities|FlowControl|DoN (+ _cyclecount 1))
    (:Exit
      (if (not (< _counter _cyclecount))
        (Class|TTBGameBoard|OnCycleComplete)
        (Utilities|Time|ClearandInvalidateTimerbyHandle (stale EventCycleonTimer _returnvalue))))))

(event EventButtonClicked
  (params (ClickedButton :type TTB%20Button%20Object%20Reference))
  ;[1 1 1] Manage gameboard win-state
  (Default|CallOnButtonsDeactivated)
  (if (== ClickedButton (Variables|Default|GetSafeButton))
    (Class|TTBGameBoard|OnLevelSuccess)
    (else
      (Class|TTBGameBoard|OnLevelFailure))))

(event EventChooseSafeButton
  (bind _safebuttonchoiceiterations (Variables|Default|GetSafeButtonChoiceIterations))
  ;[1 1 1] Precycle and safebutton selection
  (bind _outrandbutton (CallFunction|GetRandButton :!label _label))
  (if (== (Variables|Default|GetSafeButton) _outrandbutton) ; Prevent randomly selecting the same button twice in a row
    (goto _label)
    (else
      (Variables|Default|SetSafeButton _outrandbutton)
      (bind _counter (Utilities|FlowControl|DoN (+ _safebuttonchoiceiterations 1))
        (:Exit
          (if (> _counter _safebuttonchoiceiterations)
            (Utilities|Time|ClearandInvalidateTimerbyHandle (stale EventBeginPreCycle _returnvalue))
            (Class|TTBGameBoard|OnSafeButtonSet)
            (else
              (Default|FlashButton (.AsBP%20Button (Utilities|Casting|CastToBP_Button (Variables|Default|GetSafeButton))) true) ; Flash button on and off
            )))))))

(event EventOnLevelSuccess
  ;[1 1 1] Manage gameboard win-state
  (Default|FadeSafein (.AsBP%20Button (Utilities|Casting|CastToBP_Button (Variables|Default|GetSafeButton))))
  (Utilities|FlowControl|Delay 0.5)
  (for _array_element (CallFunction|GetAllButtons)
    (Default|RetractButton _array_element)
    (Default|FadeSafein _array_element))
  (Audio|SpawnSoundAttached "/Game/Sounds/SC_WindDown.SC_WindDown" (VehicleSound|GetRootComponent) "None" "0, 0, 0" "0, 0, 0" "KeepRelativeOffset" false 1.0 1.0 0.14)
  (Default|OnStageSucess (.AsBP%20Game%20Mode (Utilities|Casting|CastToBP_GameMode (Game|GetGameMode)))))

(event EventOnLevelFailure
  ;[1 1 1] Manage gameboard win-state
  (Default|FadeSafein (.AsBP%20Button (Utilities|Casting|CastToBP_Button (Variables|Default|GetSafeButton))))
  (for _array_element (CallFunction|GetAllButtons) ; Retract all buttons except the safe button.
    (if (!= _array_element (Variables|Default|GetSafeButton))
      (Default|RetractButton _array_element)))
  (Class|TTBGameBoard|DeactivateBoard)
  (Utilities|FlowControl|Delay 1.0)
  (Class|TTBGameBoard|Explode)
  (Utilities|FlowControl|Delay 1.0)
  (Default|OnStageFailed (.AsBP%20Game%20Mode (Utilities|Casting|CastToBP_GameMode (Game|GetGameMode)))))

(event EventOnSafeButtonSet
  (bind _countdownseconds (Variables|Default|GetCountdownSeconds))
  ;[1 1 1] Precycle and safebutton selection
  (Default|FlashButton (.AsBP%20Button (Utilities|Casting|CastToBP_Button (Variables|Default|GetSafeButton))) false) ; Flash on
  (bind _returnvalue (Audio|SpawnSoundAttached "/Game/Sounds/SC_MachineNoises.SC_MachineNoises" (VehicleSound|GetRootComponent) "None" "0, 0, 0" "0, 0, 0" "SnapToTarget")) ; Start machine sounds
  (bind _output_get (Variables|Default|SetMachineNoiseSoundCue _returnvalue))
  (Audio|Components|Audio|FadeIn _output_get 1.0 1.0 0.0 :!class /Script/Engine.AudioComponent) ; ..and fade the sound in
  (Default|BeginCountdown (CallFunction|GetHud) _countdownseconds) ; Start the HUD countdown
  (Utilities|FlowControl|Delay (Math|Conversions|ToFloat(Integer) _countdownseconds))
  (Class|TTBGameBoard|BeginCycle))

(event EventExplode
  ;[1 1 1] Explode gameboard
  (Audio|PlaySound2D "/Game/Sounds/SC_Hurt.SC_Hurt") ; Play player hurt sound
  (Audio|SpawnSoundAttached "/Game/Sounds/SC_Explosion.SC_Explosion" (VehicleSound|GetRootComponent)) ; Play explosion sound
  (Effects|SpawnEmitterAttached "/Game/Particles/P_Explosion.P_Explosion" (VehicleSound|GetRootComponent) "None" "0, 0, 0" "0, 0, 0" "1.000000,1.000000,1.000000" "SnapToTarget")
  (Effects|SpawnEmitterAttached "/Game/Particles/P_Smoke.P_Smoke" (VehicleSound|GetRootComponent) "None" "0, 0, 0" "0, 0, 0" "1.000000,1.000000,1.000000" "SnapToTarget")
  (Effects|SpawnEmitterAttached "/Game/Particles/P_Fire.P_Fire" (VehicleSound|GetRootComponent) "None" "0, 0, 0" "0, 0, 0" "1.000000,1.000000,1.000000" "SnapToTarget"))

(event EventBeginCycle
  ;[1 1 1] Manage button cycling
  (Variables|Default|SetBoardState "BS_Cycle")
  (Class|TTBGameBoard|CycleonTimer)
  (Default|SlowFadeOut (.AsBP%20Button (Utilities|Casting|CastToBP_Button (Variables|Default|GetSafeButton)))))

(event EventCycleonTimer
  (bind _gameboarddata (Variables|Default|GetGameboardData))
  (bind _cyclecount (Utilities|Struct|BreakGameboardData _gameboarddata))
  ;[1 1 1] Manage button cycling
  (bind _returnvalue (Utilities|Time|SetTimerbyEvent (delegate Custom|Cycle) (/ 1.0 (Class|TTBGameBoard|GetGameboardTimeScale)) true))
  (Utilities|FlowControl|DoN (+ _cyclecount 1)) ; enters at Reset
)

(event EventOnCycleComplete
  ;[1 1 1] Manage button cycling
  (Variables|Default|SetBoardState "BS_PostCycle")
  (Default|OnCycleComplete (CallFunction|GetHud))
  (Audio|Components|Audio|FadeOut (Variables|Default|GetMachineNoiseSoundCue) 1.0 0.0 :!class /Script/Engine.AudioComponent) ; Stop the machine noises
  (Default|CallOnButtonsActivated))

(event EventBeginPreCycle
  (bind _safebuttonchoiceiterations (Variables|Default|GetSafeButtonChoiceIterations))
  ;[1 1 1] Precycle and safebutton selection
  (Variables|Default|SetBoardState "BS_PreCycle")
  (bind _returnvalue (Utilities|Time|SetTimerbyEvent (delegate EventChooseSafeButton) 0.1 true))
  (Utilities|FlowControl|DoN (+ _safebuttonchoiceiterations 1)) ; enters at Reset
)

(fn ConstructionScript
  (bind _gameboarddata (Variables|Default|GetGameboardData))
  (bind (_cols _rows) (Utilities|Struct|BreakGameboardData _gameboarddata))
  (Utilities|FlowControl|Sequence
    (:then_0
      ;[1 1 1] Create buttons
      (for _index (range 0 (- (Utilities|Struct|BreakGameboardData (Variables|Default|GetGameboardData)) 1)) ; Columns
        (for _index_2 (range 0 (- (Utilities|Struct|BreakGameboardData (Variables|Default|GetGameboardData)) 1)) ; Rows
          (bind _returnvalue (AddComponent|AddChildActorComponent false (Math|Transform|MakeTransform (Math|Vector|MakeVector (- (* (* _index_2 (Variables|Default|GetButtonSpacing)) 1.0) (/ (Class|TTBGameBoard|GetBoardLength) 2.0)) (- (* _index (Variables|Default|GetButtonSpacing)) (/ (Class|TTBGameBoard|GetBoardWidth) 2.0)) (Variables|Default|GetButtonHeight)) "0, 0, 0" "1,1,1")))
          (Variables|/Game/Blueprint/BP_Button.BP_Button_C|SetGameBoard (.AsBP%20Button (Utilities|Casting|CastToBP_Button (Variables|/Script/Engine.ChildActorComponent|GetChildActor _returnvalue))) self)
          (Utilities|Array|AddUnique (LocalVariables|GetNewRow) (.AsBP%20Button (Utilities|Casting|CastToBP_Button (Variables|/Script/Engine.ChildActorComponent|GetChildActor _returnvalue)))))
        (Utilities|Array|Add (Variables|Default|GetButtonsGrid_0) (Utilities|Struct|MakeButtonGridOLD (LocalVariables|GetNewRow)))
        (Utilities|Array|Clear (LocalVariables|GetNewRow)))
      (Default|CallOnButtonGridUpdated))
    (:then_1
      ;[1 1 1] Create game board
      (for _index_3 (range 0 3) ; Build outer geometry clockwise from the top left corner
        (bind _returnvalue_2 (AddComponent|AddStaticMeshComponent false (Math|Transform|MakeTransform (* (Utilities|Select :Index _index_3 :Option%200 "-1.000000,-1.000000,0" :Option%201 "1.000000,-1.000000,0" :Option%202 "1.000000,1.000000,0" :Option%203 "-1.000000,1.000000,0") (+ (/ (Math|Vector|MakeVector (Class|TTBGameBoard|GetBoardLength) (Class|TTBGameBoard|GetBoardWidth) 0.0) 2.0) (Math|Conversions|ToVector(Float) (/ (Variables|Default|GetButtonSpacing) 2.0)))) (Math|Rotator|MakeRotator 0.0 0.0 (* _index_3 9e+01))))) ; Build corners
        (for _index_4 (range 0 (- (Utilities|Select :Index _index_3 :Option%200 _rows :Option%201 _cols :Option%202 _rows :Option%203 _cols) 1))
          (bind _returnvalue_3 (AddComponent|AddStaticMeshComponent false (Math|Transform|MakeTransform (+ (* (Math|Vector|GetRightVector (.rotation (Transformation|GetSocketTransform _returnvalue_2 "Attach" "RTS_World"))) (* _index_4 (Variables|Default|GetButtonSpacing))) (.location (Transformation|GetSocketTransform _returnvalue_2 "Attach" "RTS_World"))) (.rotation (Transformation|GetSocketTransform _returnvalue_2 "Attach" "RTS_World")) (.scale (Transformation|GetSocketTransform _returnvalue_2 "Attach" "RTS_World"))))) ; Build Walls
          (bind _returnvalue_4 (AddComponent|AddChildActorComponent false)) ; Build Gates
          (Utilities|Array|Add (Variables|Default|GetGates) (.AsBP%20Gate%20Actor (Utilities|Casting|CastToBP_GateActor (Variables|/Script/Engine.ChildActorComponent|GetChildActor _returnvalue_4))))
          (Variables|/Game/Blueprint/BP_GateActor.BP_GateActor_C|SetGameBoard (.AsBP%20Gate%20Actor (Utilities|Casting|CastToBP_GateActor (Variables|/Script/Engine.ChildActorComponent|GetChildActor _returnvalue_4))) self)
          (Class|Actor|AttachRootComponentto (.AsBP%20Gate%20Actor (Utilities|Casting|CastToBP_GateActor (Variables|/Script/Engine.ChildActorComponent|GetChildActor _returnvalue_4))) _returnvalue_3 "Attach" "SnapToTarget" true))))))

(fn GetRandButton
  (bind _gameboarddata (Variables|Default|GetGameboardData))
  (bind (_cols _rows) (Utilities|Struct|BreakGameboardData _gameboarddata))
  (return (CallFunction|GetButtonbyIndex (Math|Random|RandomIntegerinRange 0 (- _cols 1)) (Math|Random|RandomIntegerinRange 0 (- _rows 1)))))

(fn CycleButtons
  (bind _safebutton (Variables|Default|GetSafeButton))
  (bind _gameboarddata (Variables|Default|GetGameboardData))
  (bind (_cols _rows) (Utilities|Struct|BreakGameboardData _gameboarddata))
  (bind _asbp_button (Utilities|Casting|CastToBP_Button _safebutton))
  (bind (_outcolumn _outrow) (CallFunction|GetButtonIndex _asbp_button))
  (LocalVariables|SetCycleGridSectionType (Utilities|Enum|ByteToEnumGridSectionType (Math|Conversions|ToByte(Integer) (Math|Random|RandomIntegerinRange 0 1)))) ; Randomly choose to cycle columns or rows
  (LocalVariables|SetSafeButtonSectionIndex (Utilities|Select :Index (LocalVariables|GetCycleGridSectionType) :NewEnumerator0 _outcolumn :NewEnumerator1 _outrow))
  (for _index (range 1 (Utilities|Struct|BreakGameboardData (Variables|Default|GetGameboardData)))
    ;[1 1 1] Get grid section indices to move this cycle, biased towards adding a section with the safe button in it
    (bind _output_get (LocalVariables|SetNewSectionIndex (Math|Random|RandomIntegerinRange 0 (- (Utilities|Select :Index (LocalVariables|GetCycleGridSectionType) :NewEnumerator0 _cols :NewEnumerator1 _rows) 1)) :!label _label))
    (if (Utilities|Array|ContainsItem (LocalVariables|GetSelectedSections) _output_get) ; We are cycling multiple columns or rows.  If our random NewSectionIndex has already been selected, loop around and get a new random index
      (goto _label)
      (else
        (Utilities|Array|Add (LocalVariables|GetSelectedSections) (LocalVariables|GetNewSectionIndex)))))
  (Utilities|FlowControl|Sequence
    (:then_0
      ;[1 1 1] Bias the system towords including the safe buttons section
      (if (not (Utilities|Array|ContainsItem (LocalVariables|GetSelectedSections) (LocalVariables|GetSafeButtonSectionIndex))) ; If selected sections do not contain a section with the safe button in it...
        (if (< (Math|Random|RandomIntegerinRange 0 (- (Utilities|Select :Index (LocalVariables|GetCycleGridSectionType) :NewEnumerator0 _cols :NewEnumerator1 _rows) 1)) (Variables|Default|GetSafeButtonCycleBias)) ; Add a chance to forcibly set the first selected section to be the safe buttons section
          (Utilities|Array|SetArrayElem (LocalVariables|GetSelectedSections) 0 (LocalVariables|GetSafeButtonSectionIndex)))))
    (:then_1
      ;[1 1 1] Call CycleButton for each selected button and update the grid
      (for _array_element (LocalVariables|GetSelectedSections) ; For each random section
        (LocalVariables|SetCycleDirection (Utilities|Enum|ByteToEnumDirection (Math|Conversions|ToByte(Integer) (Math|Random|RandomIntegerinRange 0 1)))) ; Randomly choose a direction to cycle in
        (for (_array_element_2 _array_index) (Utilities|Select :Index (LocalVariables|GetCycleGridSectionType) :NewEnumerator0 (CallFunction|GetColumn _array_element) :NewEnumerator1 (CallFunction|GetRow _array_element)) ; For each button selected in the curren section...
          (CallFunction|PrepButtonCycle (LocalVariables|GetCycleGridSectionType) (LocalVariables|GetCycleDirection) (|IsThisButtonTravellingOffTheBoard (Utilities|Select :Index (LocalVariables|GetCycleGridSectionType) :NewEnumerator0 (CallFunction|GetColumn _array_element) :NewEnumerator1 (CallFunction|GetRow _array_element)) _array_index (LocalVariables|GetCycleDirection)) _array_element_2))
        (CallFunction|CycleGridSection _array_element (LocalVariables|GetCycleDirection) (LocalVariables|GetCycleGridSectionType)) ; Update our grid array to account for new button positions
        (Default|CallOnButtonGridUpdated) ; Broadcast grid update event.  Buttons use this for debug text if bDrawDebug is enabled in the button
        (Default|PlayGateAnim (.AsBP%20Gate%20Actor (Utilities|Casting|CastToBP_GateActor (Utilities|Array|Get(acopy) (Variables|Default|GetGates) (.Gate1 (|Getgateindicesfortheselectedsection _array_element))))))))))

(fn GetButtonbyIndex
  (params (Col :type Integer) (Row :type Integer))
  (return (Utilities|Array|Get(acopy) (.rows (Utilities|Array|Get(acopy) (Variables|Default|GetButtonsGrid_0) Col)) Row)))

(fn GetColumn
  (params (Index :type Integer))
  (return (.rows (Utilities|Array|Get(acopy) (Variables|Default|GetButtonsGrid_0) Index))))

(fn GetRow
  (params (Index :type Integer))
  (for _array_element (Variables|Default|GetButtonsGrid_0)
    (Utilities|Array|Add (LocalVariables|GetNewRow) (Utilities|Array|Get(acopy) (.rows _array_element) Index)))
  (return (LocalVariables|GetNewRow)))

(fn CycleGridSection
  (params (Idx :type Integer) (Dir :type Direction%20Enum :default "NewEnumerator0") (SectionType :type GridSectionType%20Enum :default "NewEnumerator0"))
  ;[1 1 1] Save the wires
  (LocalVariables|SetSectionIndex Idx)
  (LocalVariables|SetMovementDirection Dir)
  (LocalVariables|SetGridSectionType SectionType)
  (Utilities|FlowControl|Sequence
    (:then_0
      ;[1 1 1] Create a temporary array of our column/row
      (LocalVariables|SetNewSection (Utilities|Select :Index (LocalVariables|GetGridSectionType) :NewEnumerator0 (CallFunction|GetColumn (LocalVariables|GetSectionIndex)) :NewEnumerator1 (CallFunction|GetRow (LocalVariables|GetSectionIndex)))))
    (:then_1
      ;[1 1 1] Sort the temp array based on the direction the button elements are scrolling
      (switch Utilities|FlowControl|Switch|SwitchonDirection (LocalVariables|GetMovementDirection)
        (:NewEnumerator0
          (Utilities|Array|Insert (LocalVariables|GetNewSection) (Utilities|Array|Get(acopy) (LocalVariables|GetNewSection) (Utilities|Array|LastIndex (LocalVariables|GetNewSection)))) ; Insert the last element into the first index, pushing other indices forward
          (Utilities|Array|RemoveIndex (LocalVariables|GetNewSection) (Utilities|Array|LastIndex (LocalVariables|GetNewSection))) ; ...and remove the last element as it is now a duplicate
        )
        (:NewEnumerator1
          (Utilities|Array|Add (LocalVariables|GetNewSection) (Utilities|Array|Get(acopy) (LocalVariables|GetNewSection))) ; Add a reference of the first element to the end of the array
          (Utilities|Array|RemoveIndex (LocalVariables|GetNewSection)) ; ...and remove the first index as it is now a duplicate
        )))
    (:then_2
      ;[1 1 1] Assign the temp array back to the grid
      (switch Utilities|FlowControl|Switch|SwitchonGridSectionType (LocalVariables|GetGridSectionType)
        (:NewEnumerator0
          (Utilities|Array|SetArrayElem (Variables|Default|GetButtonsGrid_0) (LocalVariables|GetSectionIndex) (Utilities|Struct|MakeButtonGridOLD (LocalVariables|GetNewSection))))
        (:NewEnumerator1
          (for (_array_element _array_index) (LocalVariables|GetNewSection)
            (LocalVariables|SetExistingRow (.rows (Utilities|Array|Get(acopy) (Variables|Default|GetButtonsGrid_0) _array_index)))
            (Utilities|Array|SetArrayElem (LocalVariables|GetExistingRow) (LocalVariables|GetSectionIndex) _array_element)
            (Utilities|Array|SetArrayElem (Variables|Default|GetButtonsGrid_0) _array_index (Utilities|Struct|MakeButtonGridOLD (LocalVariables|GetExistingRow)))))))))

(fn GetAllButtons
  (for _array_element (Variables|Default|GetButtonsGrid_0)
    (for _array_element_2 (.rows _array_element)
      (Utilities|Array|Add (LocalVariables|GetButtonArray) _array_element_2)))
  (return (LocalVariables|GetButtonArray)))

(fn GetButtonIndex
  (params (InButton :type BP%20Button%20Object%20Reference))
  (bind (_array_element _array_index) (Utilities|Array|ForEachLoopwithBreak (Variables|Default|GetButtonsGrid_0))
    (:LoopBody
      (for (_array_element_2 _array_index_2) (.rows _array_element)
        (if (== _array_element_2 InButton)
          (return _array_index _array_index_2) ; Button found.  Return immeadiately
        )))
    (:Completed
      (return 0 0))))

(fn PrepButtonCycle
  (params (InSectionType :type GridSectionType%20Enum :default "NewEnumerator0") (InCycleDirection :type Direction%20Enum :default "NewEnumerator0") (IsTravelingOutOfGrid :type Boolean) (InButton :type BP%20Button%20Object%20Reference))
  (bind _returnvalue (Transformation|GetActorForwardVector))
  (bind _returnvalue_2 (Transformation|GetActorRightVector))
  (LocalVariables|SetGridSection InSectionType)
  (LocalVariables|SetMovementDirection InCycleDirection)
  (LocalVariables|SetButton InButton)
  (if IsTravelingOutOfGrid ; Is this button cycling off the side of the board?
    (bind _returnvalue_3 (Game|SpawnActorfromClass "/Game/Blueprint/BP_Button.BP_Button_C" (Transformation|GetActorTransform (LocalVariables|GetButton)) "AlwaysSpawn" 0 true self 0)) ; Spawn a proxy at the buttons current transform.  We'll move this off the board instead and destroy it once its hidden
    (Default|RetractButton _returnvalue_3)
    (Default|MovetoNewSlot _returnvalue_3 (Math|Transform|MakeTransform (Math|Vector|MakeVector (.X (Math|Vector|BreakVector (Math|Vector|MakeVector (.x (+ (Transformation|GetActorLocation (LocalVariables|GetButton)) (* (Utilities|Select :Index (LocalVariables|GetGridSection) :NewEnumerator0 (Utilities|Select :Index (LocalVariables|GetMovementDirection) :NewEnumerator0 _returnvalue :NewEnumerator1 (* _returnvalue -1.0)) :NewEnumerator1 (Utilities|Select :Index (LocalVariables|GetMovementDirection) :NewEnumerator0 _returnvalue_2 :NewEnumerator1 (* _returnvalue_2 -1.0))) (Variables|Default|GetButtonSpacing)))) (.y (+ (Transformation|GetActorLocation (LocalVariables|GetButton)) (* (Utilities|Select :Index (LocalVariables|GetGridSection) :NewEnumerator0 (Utilities|Select :Index (LocalVariables|GetMovementDirection) :NewEnumerator0 _returnvalue :NewEnumerator1 (* _returnvalue -1.0)) :NewEnumerator1 (Utilities|Select :Index (LocalVariables|GetMovementDirection) :NewEnumerator0 _returnvalue_2 :NewEnumerator1 (* _returnvalue_2 -1.0))) (Variables|Default|GetButtonSpacing)))) (Variables|Default|GetButtonHeight)))) (.Y (Math|Vector|BreakVector (Math|Vector|MakeVector (.x (+ (Transformation|GetActorLocation (LocalVariables|GetButton)) (* (Utilities|Select :Index (LocalVariables|GetGridSection) :NewEnumerator0 (Utilities|Select :Index (LocalVariables|GetMovementDirection) :NewEnumerator0 _returnvalue :NewEnumerator1 (* _returnvalue -1.0)) :NewEnumerator1 (Utilities|Select :Index (LocalVariables|GetMovementDirection) :NewEnumerator0 _returnvalue_2 :NewEnumerator1 (* _returnvalue_2 -1.0))) (Variables|Default|GetButtonSpacing)))) (.y (+ (Transformation|GetActorLocation (LocalVariables|GetButton)) (* (Utilities|Select :Index (LocalVariables|GetGridSection) :NewEnumerator0 (Utilities|Select :Index (LocalVariables|GetMovementDirection) :NewEnumerator0 _returnvalue :NewEnumerator1 (* _returnvalue -1.0)) :NewEnumerator1 (Utilities|Select :Index (LocalVariables|GetMovementDirection) :NewEnumerator0 _returnvalue_2 :NewEnumerator1 (* _returnvalue_2 -1.0))) (Variables|Default|GetButtonSpacing)))) (Variables|Default|GetButtonHeight)))) 0.0) (Utilities|Select :Index (LocalVariables|GetGridSection) :NewEnumerator0 (Utilities|Select :Index (LocalVariables|GetMovementDirection) :NewEnumerator0 "-90.000000,0,0.000000" :NewEnumerator1 "90.000000,0,0.000000") :NewEnumerator1 (Utilities|Select :Index (LocalVariables|GetMovementDirection) :NewEnumerator0 "0,0,90.000000" :NewEnumerator1 "0,0,-90.000000"))))
    (Transformation|SetActorLocationAndRotation (LocalVariables|GetButton) (Math|Vector|MakeVector (.x (+ (Transformation|GetActorLocation (LocalVariables|GetButton)) (Utilities|Select :Index (LocalVariables|GetGridSection) :NewEnumerator0 (Math|Vector|MakeVector (* (+ (Utilities|Select :Index (LocalVariables|GetGridSection) :NewEnumerator0 (Class|TTBGameBoard|GetBoardLength) :NewEnumerator1 (Class|TTBGameBoard|GetBoardWidth)) (Variables|Default|GetButtonSpacing)) (Utilities|Select :Index (LocalVariables|GetMovementDirection) :NewEnumerator0 -1.0 :NewEnumerator1 1.0)) 0.0 0.0) :NewEnumerator1 (Math|Vector|MakeVector 0.0 (* (+ (Utilities|Select :Index (LocalVariables|GetGridSection) :NewEnumerator0 (Class|TTBGameBoard|GetBoardLength) :NewEnumerator1 (Class|TTBGameBoard|GetBoardWidth)) (Variables|Default|GetButtonSpacing)) (Utilities|Select :Index (LocalVariables|GetMovementDirection) :NewEnumerator0 -1.0 :NewEnumerator1 1.0)) 0.0)))) (.y (+ (Transformation|GetActorLocation (LocalVariables|GetButton)) (Utilities|Select :Index (LocalVariables|GetGridSection) :NewEnumerator0 (Math|Vector|MakeVector (* (+ (Utilities|Select :Index (LocalVariables|GetGridSection) :NewEnumerator0 (Class|TTBGameBoard|GetBoardLength) :NewEnumerator1 (Class|TTBGameBoard|GetBoardWidth)) (Variables|Default|GetButtonSpacing)) (Utilities|Select :Index (LocalVariables|GetMovementDirection) :NewEnumerator0 -1.0 :NewEnumerator1 1.0)) 0.0 0.0) :NewEnumerator1 (Math|Vector|MakeVector 0.0 (* (+ (Utilities|Select :Index (LocalVariables|GetGridSection) :NewEnumerator0 (Class|TTBGameBoard|GetBoardLength) :NewEnumerator1 (Class|TTBGameBoard|GetBoardWidth)) (Variables|Default|GetButtonSpacing)) (Utilities|Select :Index (LocalVariables|GetMovementDirection) :NewEnumerator0 -1.0 :NewEnumerator1 1.0)) 0.0)))) 0.0) (* (Utilities|Select :Index (LocalVariables|GetGridSection) :NewEnumerator0 (Utilities|Select :Index (LocalVariables|GetMovementDirection) :NewEnumerator0 "-90.000000,0,0.000000" :NewEnumerator1 "90.000000,0,0.000000") :NewEnumerator1 (Utilities|Select :Index (LocalVariables|GetMovementDirection) :NewEnumerator0 "0,0,90.000000" :NewEnumerator1 "0,0,-90.000000")) -1.0)) ; Move the button to a position at the opposite side of the board where it will scroll in from
    (Default|RetractImmediate (LocalVariables|GetButton)) ; Retract the button immediatly as it's cycling in from off grid
    (Default|ExtendButton (LocalVariables|GetButton)))
  (Default|MovetoNewSlot (LocalVariables|GetButton) (Math|Transform|MakeTransform (Math|Vector|MakeVector (.x (+ (Transformation|GetActorLocation (LocalVariables|GetButton)) (* (Utilities|Select :Index (LocalVariables|GetGridSection) :NewEnumerator0 (Utilities|Select :Index (LocalVariables|GetMovementDirection) :NewEnumerator0 _returnvalue :NewEnumerator1 (* _returnvalue -1.0)) :NewEnumerator1 (Utilities|Select :Index (LocalVariables|GetMovementDirection) :NewEnumerator0 _returnvalue_2 :NewEnumerator1 (* _returnvalue_2 -1.0))) (Variables|Default|GetButtonSpacing)))) (.y (+ (Transformation|GetActorLocation (LocalVariables|GetButton)) (* (Utilities|Select :Index (LocalVariables|GetGridSection) :NewEnumerator0 (Utilities|Select :Index (LocalVariables|GetMovementDirection) :NewEnumerator0 _returnvalue :NewEnumerator1 (* _returnvalue -1.0)) :NewEnumerator1 (Utilities|Select :Index (LocalVariables|GetMovementDirection) :NewEnumerator0 _returnvalue_2 :NewEnumerator1 (* _returnvalue_2 -1.0))) (Variables|Default|GetButtonSpacing)))) (Variables|Default|GetButtonHeight)) "0, 0, 0" "1,1,1")))

(fn GetHud
  (return (.AsBP%20HUD (Utilities|Casting|CastToBP_HUD (HUD|GetHUD (Game|GetPlayerController 0))))))