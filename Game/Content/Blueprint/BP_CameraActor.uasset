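; Camera actor that automatically frames a focus target, which is set through SetFocusTarget, by centring and zooming on it.
; Each Tick projects the target's eight bounding-box corners into a screen rectangle, skipping the update if any projection fails.
; The larger rectangle-to-viewport ratio, with margin, scales spring arm length, while the deprojected offset from screen centre moves the actor, both interpolated.
; GetBoundingBox and GetFrustrumWidthAtDistance are uncalled helpers.
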(event `SetFocusTarget`
  (params (TargetActor :type "Actor Object Reference"))
  (set `self.FocusTarget` TargetActor))

(event `self.ReceiveTick`
  (params (DeltaSeconds :type "Float (single-precision)"))
  (bind (_returnvalue_x _returnvalue_y) (`KismetMathLibrary.BreakVector2D` (`WidgetLayoutLibrary.GetViewportSize`)))
  (bind _returnvalue (`self.K2_GetActorLocation`))
  (bind _returnvalue_x_2 (`KismetMathLibrary.BreakVector2D` (`WidgetLayoutLibrary.GetViewportSize`)))
  (bind (_box_min _box_max) (break `Box2D` (`self.Box`)))
  (bind (_box_min_2 _box_max_2) (break `Box2D` (`self.Box`)))
  (bind (_allpointsconverted _outbox2d) (`self.Get2DBoundingRectangle` (`self.FocusTarget`)))
  (bind (_returnvalue_x_3 _returnvalue_y_2) (`KismetMathLibrary.BreakVector2D` (+ (- _box_max _box_min) (`self.ZoomMargin`))))
  (`/Engine/EditorBlueprintResources/StandardMacros.IsValid` (`self.FocusTarget`)
    (:`Is Valid`
      (set `self.Box` _outbox2d)
      (if _allpointsconverted
        (set `SpringArmComponent.TargetArmLength` (`KismetMathLibrary.FInterpTo` (`SpringArmComponent.TargetArmLength` (`self.SpringArm`)) (* (`SpringArmComponent.TargetArmLength` (`self.SpringArm`)) (`KismetMathLibrary.FMax` (/ _returnvalue_y_2 _returnvalue_y) (/ _returnvalue_x_3 _returnvalue_x_2))) (`GameplayStatics.GetWorldDeltaSeconds`) 2.0) (`self.SpringArm`))
        (`self.K2_SetActorLocation` (`KismetMathLibrary.VInterpTo` _returnvalue (+ _returnvalue (- (`GameplayStatics.DeprojectScreenToWorld` (`GameplayStatics.GetPlayerController` 0) (/ (+ _box_min_2 _box_max_2) 2.0)) (`GameplayStatics.DeprojectScreenToWorld` (`GameplayStatics.GetPlayerController` 0) (/ (`WidgetLayoutLibrary.GetViewportSize`) 2.0)))) (`GameplayStatics.GetWorldDeltaSeconds`) 20.0))))))

(fn `Get2DBoundingRectangle`
  (params (Actor :type "Actor Object Reference"))
  (returns (AllPointsConverted :type Boolean) (OutBox2D :type "Box2D Structure"))
  (locals (ScreenSpacePoints :type "Array of Vector2D Structure") (TopLeft :type "Vector2D Structure") (BottomRight :type "Vector2D Structure") (Total :type "Vector2D Structure") (Average :type "Vector2D Structure") (BoxOrigin :type "Vector2D Structure") (Box2D :type "Box2D Structure"))
  (bind (_origin _boxextent) (`self.GetActorBounds` Actor false))
  (bind _box2d (`local.Box2D`))
  (for _array_element (`self.GetBoundingBoxPoints` _origin _boxextent)
    (bind (_screenposition _returnvalue) (`GameplayStatics.ProjectWorldToScreen` (`GameplayStatics.GetPlayerController` 0) _array_element))
    (if _returnvalue
      (`KismetArrayLibrary.Array_Add` (`local.ScreenSpacePoints`) _screenposition)
      (set `local.Total` (+ (`local.Total`) _screenposition))
      (else
        (return false))))
  (set `local.Box2D` (make `Box2D` (`|GetArrayItem` (`local.ScreenSpacePoints`)))) ; Box2d Min needs an initial value as no new value will be smaller that the default (0, 0) value
  (for _array_element_2 (`local.ScreenSpacePoints`)
    (bind (_x _y) (`KismetMathLibrary.BreakVector2D` _array_element_2))
    (set `local.Box2D` (make `Box2D` (`KismetMathLibrary.MakeVector2D` (`KismetMathLibrary.FMin` (`KismetMathLibrary.BreakVector2D` (break `Box2D` _box2d)) _x) (`KismetMathLibrary.FMin` (`.Y` (`KismetMathLibrary.BreakVector2D` (break `Box2D` _box2d))) _y)) (`KismetMathLibrary.MakeVector2D` (`KismetMathLibrary.FMax` (`KismetMathLibrary.BreakVector2D` (`.Max` (break `Box2D` _box2d))) _x) (`KismetMathLibrary.FMax` (`.Y` (`KismetMathLibrary.BreakVector2D` (`.Max` (break `Box2D` _box2d)))) _y)))))
  (set `local.BoxOrigin` (/ (+ (`local.TopLeft`) (`local.BottomRight`)) 2.0)) ; Origin is the average position of all points
  (return true (`local.Box2D`)))

(fn `GetBoundingBox`
  (params (TargetActor :type "Actor Object Reference") (Transform :type "Transform Structure"))
  (returns (Extents :type "Vector Structure") (OriginTransform :type "Transform Structure"))
  (locals (BBPoints :type "Array of Vector Structure"))
  (bind (_origin _boxextent) (`self.GetActorBounds` TargetActor false))
  (bind _returnvalue (`KismetMathLibrary.GetForwardVector` (.rotation Transform)))
  (for _array_element (`self.GetBoundingBoxPoints` _origin _boxextent)
    (`KismetArrayLibrary.Array_Add` (`local.BBPoints`) (`KismetMathLibrary.InverseTransformLocation` Transform (`.Intersection` (`KismetMathLibrary.LinePlaneIntersection_OriginNormal` (+ _array_element (* _returnvalue -500.0)) (+ _array_element (* _returnvalue 500.0)) (.location Transform) _returnvalue)))))
  (return (0.0 0.0 0.0) (`KismetMathLibrary.MakeTransform` (`KismetMathLibrary.TransformLocation` Transform) (.rotation Transform))))

(fn `GetBoundingBoxPoints`
  (params (InOrigin :type "Vector Structure") (InExtents :type "Vector Structure"))
  (returns (OutPoints :type "Array of Vector Structure"))
  (locals (Origin :type "Vector Structure") (Extents :type "Vector Structure") (Points :type "Array of Vector Structure"))
  (set `local.Origin` InOrigin)
  (set `local.Extents` InExtents)
  (for _array_element (`|MakeArray` (1.0 1.0 1.0) (-1.0 1.0 1.0) (-1.0 -1.0 1.0) (1.0 -1.0 1.0) (1.0 1.0 -1.0) (-1.0 1.0 -1.0) (-1.0 -1.0 -1.0) (1.0 -1.0 -1.0) :!type "Vector Structure")
    (`KismetArrayLibrary.Array_Add` (`local.Points`) (+ (* _array_element (`local.Extents`)) (`local.Origin`))))
  (return (`local.Points`)))

(fn `GetFrustrumWidthAtDistance`
  (params (Distance :type "Float (double-precision)"))
  (locals (Width :type "Float (double-precision)"))
  (bind (_returnvalue_location _returnvalue_rotation) (`KismetMathLibrary.BreakTransform` (`SceneComponent.K2_GetComponentToWorld` (`self.Camera`))))
  (bind _returnvalue (+ _returnvalue_location (* (`KismetMathLibrary.GetForwardVector` _returnvalue_rotation) Distance)))
  (set `local.Width` (* (* 2.0 Distance) (`KismetMathLibrary.DegreesToRadians` (* 0.5 (`CameraComponent.FieldOfView` (`self.Camera`))))))
  (`KismetSystemLibrary.DrawDebugLine` _returnvalue (+ _returnvalue (* (`KismetMathLibrary.GetRightVector` _returnvalue_rotation) (* (`local.Width`) 0.5))) (struct :`R` 1.0 :`G` 0.909158 :`B` 0.039792 :`A` 1.0) 0.0 0.2))

(fn `UserConstructionScript`)